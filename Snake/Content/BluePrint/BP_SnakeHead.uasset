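; Snake head actor for a grid-based Snake game, turned left or right by input and sped up while a key is held.
; A looping, delay-timed step passes its position down a linked chain of body segments, moves along an indexed direction array, rotates, then calls the body's head-collision check.
; Overlapping food destroys it, appends a new body segment and has the GameMode spawn more; a local recursive CreateFood is unused here.
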(event `self.ReceiveActorBeginOverlap`
  (params (OtherActor :type "Actor Object Reference"))
  (bind _asbp_food (cast `/Game/BluePrint/BP_Food` OtherActor))
  (`/Engine/EditorBlueprintResources/StandardMacros.IsValid` _asbp_food
    (:`Is Valid`
      (`self.K2_DestroyActor` _asbp_food)
      (`self.CreateSnakeBody`)
      (bind _asbp_game_mode (cast `/Game/BluePrint/BP_GameMode` (`GameplayStatics.GetGameMode`)))
      (`/Game/BluePrint/BP_GameMode.CreateFood` _asbp_game_mode)
      (bind _asbp_game_state (cast `/Game/BluePrint/BP_GameState` (`GameplayStatics.GetGameState`))))))

(event `self.ReceiveBeginPlay`
  (`self.MoveWork` :!label _label))

(event `MoveWork`
  (`self.UpdateBodyPos`)
  (`self.K2_AddActorWorldOffset` (* (`self.GetSnakeDirection`) 100))
  (`self.UdpateRotate`)
  (set `self.CurrentStepIndex` (`self.DirIndex`))
  (`self.CheckBodyPos`)
  (`KismetSystemLibrary.Delay` (`self.Get Move Speed`))
  (goto _label))

(event `InputAction|TurnRight`
  (params (Key :type "Key Structure"))
  (:`Pressed`
    (`self.SnakeTurnRightFunc`)))

(event `InputAction|TurnLeft`
  (params (Key :type "Key Structure"))
  (:`Pressed`
    (`self.SnakeTurnLeftFunc`)))

(event `InputAction|UpSpeed`
  (params (Key :type "Key Structure"))
  (:`Pressed`
    (set `self.IsUPSpeed` true))
  (:`Released`
    (set `self.IsUPSpeed` false)))

(fn `AddSnakeBody`
  (params (NextBody :type "/Game/BluePrint/BP_SnakeBody Object Reference"))
  (`/Engine/EditorBlueprintResources/StandardMacros.IsValid` (`self.NextSnakeBody`)
    (:`Is Valid`
      (`/Game/BluePrint/BP_SnakeBody.AddSnakeBody` (`self.NextSnakeBody`) NextBody))
    (:`Is Not Valid`
      (bind _output_get (set `self.NextSnakeBody` NextBody))
      (`self.K2_SetActorLocation` _output_get (+ (`self.K2_GetActorLocation`) (* (`self.GetSnakeDirection`) -100)) false false)
      (set `/Game/BluePrint/BP_SnakeBody.MoveDir` (`self.MoveDir`) _output_get))))

(fn `CheckBodyPos`
  (`/Engine/EditorBlueprintResources/StandardMacros.IsValid` null
    (:`Is Valid`
      (`/Game/BluePrint/BP_SnakeBody.CheckCollisionHead` (`self.NextSnakeBody`) (`self.K2_GetActorLocation`)))))

(fn `CreateFood`
  (params (NewParam :type Integer))
  (locals (RandomPos :type "Vector Structure"))
  (`KismetSystemLibrary.PrintString` (`KismetStringLibrary.Conv_IntToString` NewParam))
  (set `local.RandomPos` (`KismetMathLibrary.MakeVector` (* (- (`KismetMathLibrary.RandomIntegerFromStream` 20 (`self.RandomSeed`)) 10) 100.0) (* (- (`KismetMathLibrary.RandomIntegerFromStream` 20 (`self.RandomSeed`)) 10) 100.0)))
  (bind (_outhit _returnvalue) (`KismetSystemLibrary.SphereTraceSingle` (`local.RandomPos`) (`local.RandomPos`) 40.0 "TraceTypeQuery1"))
  (if _returnvalue
    (`KismetSystemLibrary.PrintString` "Find")
    (`self.CreateFood` (+ NewParam 1))
    (else
      (`KismetSystemLibrary.PrintString` "NoFind")
      (`|SpawnActorFromClass` "/Game/BluePrint/BP_Food.BP_Food_C" (`KismetMathLibrary.MakeTransform` (`local.RandomPos`)) "Undefined" "OverrideRootScale" null null))))

(fn `CreateSnakeBody`
  (bind _returnvalue (`|SpawnActorFromClass` "/Game/BluePrint/BP_SnakeBody.BP_SnakeBody_C" (`KismetMathLibrary.MakeTransform` (0.0 0.0 0.0)) "Undefined" "OverrideRootScale" null null))
  (`self.AddSnakeBody` _returnvalue))

(fn `Get Move Speed`
  (returns (DelayTime :type "Float (double-precision)"))
  (if (`self.IsUPSpeed`)
    (return 0.4)
    (else
      (return 0.8))))

(fn `GetSnakeDirection`
  (returns (Direction :type "Vector Structure"))
  (if (< (`self.DirIndex`) 0)
    (set `self.DirIndex` 0))
  (if (>= (`self.DirIndex`) (`KismetArrayLibrary.Array_Length` (`self.ConstMoveDir`)))
    (set `self.DirIndex` 0))
  (return (`|GetArrayItem` (`self.ConstMoveDir`) (`self.DirIndex`))))

(fn `SnakeTurnLeftFunc`
  (locals (NextTempIndex :type Integer))
  (bind _output_get (set `local.NextTempIndex` (- (`self.CurrentStepIndex`) 1)))
  (if (< _output_get 0)
    (set `self.DirIndex` (- (`KismetArrayLibrary.Array_Length` (`self.ConstMoveDir`)) 1))
    (else
      (set `self.DirIndex` (`local.NextTempIndex`)))))

(fn `SnakeTurnRightFunc`
  (locals (NextTempIndex :type Integer))
  (bind _output_get (set `local.NextTempIndex` (+ (`self.CurrentStepIndex`) 1)))
  (if (>= _output_get (`KismetArrayLibrary.Array_Length` (`self.ConstMoveDir`)))
    (set `self.DirIndex` 0)
    (else
      (set `self.DirIndex` (`local.NextTempIndex`)))))

(fn `UdpateRotate`
  (locals (NowDir :type "Vector Structure"))
  (bind (_nowdir_x _nowdir_y _nowdir_z) (`KismetMathLibrary.BreakVector` (`local.NowDir`)))
  (switch `int` (`self.DirIndex`)
    (:`0`
      (set `local.NowDir` (0.0 0.0 0.0))
      (`KismetSystemLibrary.PrintString` "前"))
    (:`1`
      (set `local.NowDir` (0.0 0.0 90.0))
      (`KismetSystemLibrary.PrintString` "右"))
    (:`2`
      (set `local.NowDir` (0.0 0.0 180.0))
      (`KismetSystemLibrary.PrintString` "后"))
    (:`3`
      (set `local.NowDir` (0.0 0.0 -90.0))
      (`KismetSystemLibrary.PrintString` "左")))
  (`self.K2_SetActorRotation` (`KismetMathLibrary.MakeRotator` _nowdir_x _nowdir_y _nowdir_z)))

(fn `UpdateBodyPos`
  (bind _nextsnakebody (`self.NextSnakeBody`))
  (`/Engine/EditorBlueprintResources/StandardMacros.IsValid` _nextsnakebody
    (:`Is Valid`
      (`/Game/BluePrint/BP_SnakeBody.UpdateBodyPos` _nextsnakebody (`self.GetSnakeDirection`) (`self.K2_GetActorLocation`)))))

(fn `UserConstructionScript`)