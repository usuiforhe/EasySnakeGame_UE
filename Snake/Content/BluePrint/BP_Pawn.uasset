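; BP_Pawn is a pawn in a snake game that toggles the player's view between itself and the snake head.
; The ChangeViewer input drives a FlipFlop that alternately blends the first player controller's view target to the first valid BP_SnakeHead found and back to this pawn.
; The construction script pins the pawn to a hardcoded location and rotation, giving it a fixed vantage point.
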(event `InputAction|ChangeViewer`
  (params (Key :type "Key Structure"))
  (:`Pressed`
    (`/Engine/EditorBlueprintResources/StandardMacros.FlipFlop`
      (:`A`
        (bind _outactors (`GameplayStatics.GetAllActorsOfClass` "/Game/BluePrint/BP_SnakeHead.BP_SnakeHead_C"))
        (for _array_element _outactors
          (`/Engine/EditorBlueprintResources/StandardMacros.IsValid` _array_element
            (:`Is Valid`
              (`PlayerController.SetViewTargetWithBlend` (`GameplayStatics.GetPlayerController` 0) _array_element 1.0 "VTBlend_Linear" 0.0 false)
              (break)))))
      (:`B`
        (`PlayerController.SetViewTargetWithBlend` (`GameplayStatics.GetPlayerController` 0) self 1.0 "VTBlend_Linear" 0.0 false)))))

(fn `UserConstructionScript`
  (`self.K2_SetActorTransform` (`KismetMathLibrary.MakeTransform` (506.0 -770.0 4330.0) (struct :`Pitch` -90.0 :`Yaw` 180.0 :`Roll` 180.0))))