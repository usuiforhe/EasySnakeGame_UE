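; BP_SnakeBody is one body segment of a grid-style snake, linked to the segment behind it as a recursive chain.
; New segments append at the tail, 100 units opposite its move direction.
; Position updates ripple down the chain, each segment passing its old location and direction to the next.
; A head-position check destroys the segment it overlaps along with every segment behind it.
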(fn `AddSnakeBody`
  (params (Body :type "/Game/BluePrint/BP_SnakeBody Object Reference"))
  (`/Engine/EditorBlueprintResources/StandardMacros.IsValid` (`self.NextSnakeBody`)
    (:`Is Valid`
      (`self.AddSnakeBody` (`self.NextSnakeBody`) Body))
    (:`Is Not Valid`
      (bind _output_get (set `self.NextSnakeBody` Body))
      (`self.K2_SetActorLocation` _output_get (+ (`self.K2_GetActorLocation`) (* (`self.MoveDir`) -100)) false false)
      (set `/Game/BluePrint/BP_SnakeBody.MoveDir` (`self.MoveDir`) _output_get))))

(fn `CheckCollisionHead`
  (params (HeadPos :type "Vector Structure"))
  (bind _nextsnakebody (`self.NextSnakeBody`))
  (if (== (`self.K2_GetActorLocation`) HeadPos)
    (`self.RemoveSelfAndChild`)
    (else
      (`/Engine/EditorBlueprintResources/StandardMacros.IsValid` _nextsnakebody
        (:`Is Valid`
          (`self.CheckCollisionHead` _nextsnakebody HeadPos))))))

(fn `RemoveSelfAndChild`
  (bind _nextsnakebody (`self.NextSnakeBody`))
  (`/Engine/EditorBlueprintResources/StandardMacros.IsValid` _nextsnakebody
    (:`Is Valid`
      (`self.RemoveSelfAndChild` _nextsnakebody))
    (:`Is Not Valid`
      _))
  (`self.K2_DestroyActor`))

(fn `UpdateBodyPos`
  (params (Direction :type "Vector Structure") (Pos :type "Vector Structure"))
  (locals (OldPos :type "Vector Structure") (OldMoveDIr :type "Vector Structure"))
  (bind _nextsnakebody (`self.NextSnakeBody`))
  (set `local.OldPos` (`self.K2_GetActorLocation`))
  (set `local.OldMoveDIr` (`self.MoveDir`))
  (set `self.MoveDir` Direction)
  (`self.K2_SetActorLocation` Pos)
  (`/Engine/EditorBlueprintResources/StandardMacros.IsValid` _nextsnakebody
    (:`Is Valid`
      (`self.UpdateBodyPos` _nextsnakebody (`local.OldMoveDIr`) (`local.OldPos`)))))

(fn `UserConstructionScript`)