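; BP_GameMode is a game mode Blueprint that spawns a BP_Food actor at a random free spot when play begins.
; CreateFood picks a point on a 100-unit grid around the world origin at Z zero, using the RandomSeed stream.
; A zero-length sphere trace on the Visibility channel tests that point, and the function recursively retries until it finds an unblocked one, printing debug strings for each result.
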(event `self.ReceiveBeginPlay`
  (`self.CreateFood`))

(fn `CreateFood`
  (locals (RandomPos :type "Vector Structure"))
  (set `local.RandomPos` (`KismetMathLibrary.MakeVector` (* (- (`KismetMathLibrary.RandomIntegerFromStream` 20 (`self.RandomSeed`)) 10) 100.0) (* (- (`KismetMathLibrary.RandomIntegerFromStream` 20 (`self.RandomSeed`)) 10) 100.0)))
  (bind (_outhit _returnvalue) (`KismetSystemLibrary.SphereTraceSingle` (`local.RandomPos`) (`local.RandomPos`) 40.0 "TraceTypeQuery1"))
  (if _returnvalue
    (`KismetSystemLibrary.PrintString` "Find")
    (`self.CreateFood`)
    (else
      (`KismetSystemLibrary.PrintString` "NoFind")
      (`|SpawnActorFromClass` "/Game/BluePrint/BP_Food.BP_Food_C" (`KismetMathLibrary.MakeTransform` (`local.RandomPos`)) "Undefined" "OverrideRootScale" null null))))

(fn `UserConstructionScript`)